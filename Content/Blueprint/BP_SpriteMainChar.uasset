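; Paper2D knight player character with run, jump, melee attack, hit and death flipbooks, driven by Enhanced Input movement and jump plus a left-click attack.
; Jumping blocks movement input while a Delay loop polls vertical velocity for landing.
; A Tick-checked attack frame fires a DoOnce hit check, damaging overlapping characters of its own class and spawning a flash.
; Damage subtracts fixed health, and finished animations return to idle unless dead.
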(event `self.ReceiveBeginPlay`
  ;[1 1 1] Movement_Axis
  (bind _asbp_player_controller (cast `/Game/Blueprint/BP_PlayerController` (`self.GetController`)))
  (`EnhancedInputSubsystemInterface.AddMappingContext` (pcsubsystem `EnhancedInputLocalPlayerSubsystem` _asbp_player_controller) "/Game/Blueprint/IMC_Default.IMC_Default" 0 (struct)))

(event `EnhancedInput|/Game/Blueprint/IA_Movement`
  (params (ActionValue :type "Float (double-precision)") (ElapsedSeconds :type "Float (double-precision)") (TriggeredSeconds :type "Float (double-precision)") (InputAction :type "InputAction Object Reference" :default "/Game/Blueprint/IA_Movement.IA_Movement"))
  (bind _sprite (`self.Sprite`))
  ;[1 1 1] Run-Idle
  (:`Triggered`
    (if (not (`self.BLN_Jumping`))
      (`self.AddMovementInput` (`self.GetActorForwardVector`) ActionValue)
      (`PaperFlipbookComponent.SetFlipbook` _sprite "/Game/Assests/Knight/Flipbook/_Run1._Run1")
      (if (> ActionValue 0.0)
        (`SceneComponent.K2_SetWorldRotation` :`self` _sprite)
        (else
          (`SceneComponent.K2_SetWorldRotation` _sprite (struct :`Yaw` -180.0) false false)))))
  (:`Completed`
    (if (not (`self.BLN_Jumping`))
      (`PaperFlipbookComponent.SetFlipbook` _sprite "/Game/Assests/Knight/Flipbook/Knight_Idle1.Knight_Idle1"))))

(event `EnhancedInput|/Game/Blueprint/IA_Jump`
  (params (ActionValue :type "Float (double-precision)") (ElapsedSeconds :type "Float (double-precision)") (TriggeredSeconds :type "Float (double-precision)") (InputAction :type "InputAction Object Reference" :default "/Game/Blueprint/IA_Jump.IA_Jump"))
  (bind (_returnvalue_x _returnvalue_y _returnvalue_z) (`KismetMathLibrary.BreakVector` (`self.GetVelocity`)))
  (bind _sprite (`self.Sprite`))
  ;[1 1 1] Jumping
  (:`Triggered`
    (if (not (`self.BLN_Jumping`))
      (set `self.BLN_Jumping` true)
      (`self.Jump`)
      (`PaperFlipbookComponent.SetLooping` _sprite false)
      (`PaperFlipbookComponent.SetFlipbook` _sprite "/Game/Assests/Knight/Flipbook/_Jump1._Jump1")
      (`KismetSystemLibrary.Delay` 0.1)
      (if (== _returnvalue_z 0.0) :!label _label
        (`PaperFlipbookComponent.SetLooping` _sprite false)
        (`PaperFlipbookComponent.Play` _sprite)
        (`PaperFlipbookComponent.SetFlipbook` _sprite "/Game/Assests/Knight/Flipbook/Knight_Idle1.Knight_Idle1")
        (set `self.BLN_Jumping` false)
        (else
          (`KismetSystemLibrary.Delay` 0.1)
          (goto _label))))))

(event `Key|LeftMouseButton`
  (params (Key :type "Key Structure"))
  (bind _sprite (`self.Sprite`))
  ;[1 1 1] Atk Animation
  (:`Pressed`
    (`PaperFlipbookComponent.SetFlipbook` _sprite "/Game/Assests/Knight/Flipbook/_Attack2._Attack2")
    (`PaperFlipbookComponent.SetLooping` _sprite false)
    (set `self.IsAttacking` true)))

(event `self.Sprite.OnFinishedPlaying`
  ;[1 1 1] Restart Animation
  (if (not (`self.IsDead`))
    (`PaperFlipbookComponent.SetFlipbook` (`self.Sprite`) "/Game/Assests/Knight/Flipbook/Knight_Idle1.Knight_Idle1")
    (`self.Restart_Animation`)
    (set `self.IsAttacking` false)
    (`self.resetAtk`)
    (`SceneComponent.SetHiddenInGame` (`self.Hitbox`) true false)))

(event `resetAtk`
  ;[1 1 1] Atk_Hitbox
  (goto _label_2 :!via `Reset`))

(event `self.ReceiveTick`
  (params (DeltaSeconds :type "Float (single-precision)"))
  (bind _hitbox (`self.Hitbox`))
  ;[1 1 1] Atk_Hitbox
  (if (`self.IsAttacking`)
    (if (== (`PaperFlipbookComponent.GetPlaybackPositionInFrames` (`self.Sprite`)) 12)
      (`/Engine/EditorBlueprintResources/StandardMacros.DoOnce` false :!label _label_2
        (:`Completed`
          (`self.Hit Check`)
          (`SceneComponent.SetHiddenInGame` _hitbox false false)))
      (else
        (`SceneComponent.SetHiddenInGame` _hitbox true false)))))

(event `self.ReceiveAnyDamage`
  (params (Damage :type "Float (single-precision)") (DamageType :type "DamageType Object Reference") (InstigatedBy :type "Controller Object Reference") (DamageCauser :type "Actor Object Reference"))
  (bind _sprite (`self.Sprite`))
  ;[1 1 1] Damage_Animation
  (set `self.Health` (- (`self.Health`) 50.0))
  (if (<= (`self.Health`) 0.0)
    (`PaperFlipbookComponent.SetFlipbook` _sprite "/Game/Assests/Knight/Flipbook/Knight_Death1.Knight_Death1")
    (`PaperFlipbookComponent.SetLooping` _sprite false)
    (set `self.IsDead` true)
    (else
      (`PaperFlipbookComponent.SetFlipbook` _sprite "/Game/Assests/Knight/Hit/_Hit1._Hit1")
      (`PaperFlipbookComponent.SetLooping` _sprite false))))

(fn `Hit Check`
  (locals (HitSomething :type Boolean))
  (for _array_element (`PrimitiveComponent.GetOverlappingActors` (`self.Hitbox`) "BP_SpriteMainChar_C")
    (if (!= _array_element self)
      (`GameplayStatics.ApplyDamage` _array_element (`self.DamageAmount`))
      (set `local.HitSomething` true)))
  (if (`local.HitSomething`)
    (`NiagaraFunctionLibrary.SpawnSystemAtLocation` "/Game/VFX_Niagara/Hit_Flash.Hit_Flash" (`SceneComponent.GetSocketLocation` (`self.Sprite`) "HitPos"))))

(fn `Restart_Animation`
  (bind _sprite (`self.Sprite`))
  (`PaperFlipbookComponent.SetLooping` _sprite true)
  (if (not (`PaperFlipbookComponent.IsPlaying` _sprite))
    (`PaperFlipbookComponent.Play` _sprite)))

(fn `UserConstructionScript`)